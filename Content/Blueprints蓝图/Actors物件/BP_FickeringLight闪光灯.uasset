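; BP_FickeringLight is a light actor that flickers its PointLight during play.
; The construction script sets the light to its base intensity.
; From BeginPlay, a looping RetriggerableDelay waits a random time between Min and Max, then a FlipFlop alternates the light between the minimum flicker intensity and the base intensity.
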(event `self.ReceiveBeginPlay`
  (bind _pointlight (`self.PointLight`))
  (`KismetSystemLibrary.RetriggerableDelay` (`KismetMathLibrary.RandomFloatInRange` (`self.Min`) (`self.Max`)) :!label _label)
  (`/Engine/EditorBlueprintResources/StandardMacros.FlipFlop`
    (:`A`
      (`LightComponent.SetIntensity` _pointlight (`self.MinFlickerIntensity最小闪光强度`))
      (goto _label))
    (:`B`
      (`LightComponent.SetIntensity` _pointlight (`self. Intensity强度`))
      (goto _label))))

(fn `UserConstructionScript`
  (`LightComponent.SetIntensity` (`self.PointLight`) (`self. Intensity强度`)))