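; Base pickup actor that lets the player collect an item into their inventory component.
; Sphere overlap starts per-tick updates that line-trace to the player camera, showing a camera-facing prompt widget when unobstructed.
; Distance to the camera toggles the prompt state and enables or disables the actor's interact input.
; Interacting adds the item, then keeps any remainder in the actor or destroys it when none is left.
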(event `self.Sphere.OnComponentBeginOverlap`
  (params (OverlappedComponent :type "PrimitiveComponent Object Reference") (OtherActor :type "Actor Object Reference") (OtherComp :type "PrimitiveComponent Object Reference") (OtherBodyIndex :type Integer) (bFromSweep :type Boolean) (SweepResult :type "HitResult Structure (by ref)"))
  (bind `_asl1_player_character角色` (cast `/Game/GameBP游戏蓝图/Level1关卡1/L1_PlayerCharacter角色` OtherActor))
  (set `self.PlayerRef角色映射` `_asl1_player_character角色`)
  (`SceneComponent.SetVisibility` (`self.PromptWidget提示控件`) true false)
  (set `self.UpDateActor更新物件` true))

(event `self.Sphere.OnComponentEndOverlap`
  (params (OverlappedComponent :type "PrimitiveComponent Object Reference") (OtherActor :type "Actor Object Reference") (OtherComp :type "PrimitiveComponent Object Reference") (OtherBodyIndex :type Integer))
  (cast `/Game/GameBP游戏蓝图/Level1关卡1/L1_PlayerCharacter角色` OtherActor)
  (`SceneComponent.SetVisibility` (`self.PromptWidget提示控件`) false false)
  (set `self.UpDateActor更新物件` false)
  (`self.DisableInput` (`GameplayStatics.GetPlayerController` 0)))

(event `self.ReceiveTick`
  (params (DeltaSeconds :type "Float (single-precision)"))
  (bind _returnvalue (`GameplayStatics.GetPlayerController` 0))
  (bind `_promptwidget提示控件` (`self.PromptWidget提示控件`))
  (bind (_returnvalue_x _returnvalue_y _returnvalue_z) (`KismetMathLibrary.BreakVector` (`SceneComponent.K2_GetComponentLocation` (`self.StaticMesh`))))
  (`SceneComponent.K2_SetWorldLocation` (`self.PromptWidget提示控件`) (`KismetMathLibrary.MakeVector` _returnvalue_x _returnvalue_y (+ _returnvalue_z (`self.WidgeDistance提示控件距离`))) false false)
  (if (`self.UpDateActor更新物件`)
    (bind (_outhit _returnvalue_2) (`KismetSystemLibrary.LineTraceSingle` (`self.K2_GetActorLocation`) (`SceneComponent.K2_GetComponentLocation` (`/Game/GameBP游戏蓝图/Level1关卡1/L1_PlayerCharacter角色.Camera` (`self.PlayerRef角色映射`))) "TraceTypeQuery1"))
    (if (not _returnvalue_2)
      (`SceneComponent.SetVisibility` `_promptwidget提示控件` true false)
      (`SceneComponent.K2_SetWorldRotation` (`self.PromptWidget提示控件`) (`KismetMathLibrary.FindLookAtRotation` (`SceneComponent.K2_GetComponentLocation` (`self.PromptWidget提示控件`)) (`SceneComponent.K2_GetComponentLocation` (`/Game/GameBP游戏蓝图/Level1关卡1/L1_PlayerCharacter角色.Camera` (`self.PlayerRef角色映射`)))) false false)
      (bind (_bblockinghit _binitialoverlap _time _distance _location _impactpoint _normal _impactnormal _physmat _hitactor _hitcomponent _hitbonename _bonename _hititem _elementindex _faceindex _tracestart _traceend) (`GameplayStatics.BreakHitResult` _outhit))
      (bind _returnvalue_3 (<= (`KismetMathLibrary.VSize` (- _tracestart _traceend)) (`self.PickUpDistance拾取距离`)))
      (`/Game/UMG界面/Inventory库存/W_PickupPrompt拾取提示.TogglePrompt切换提示` (cast `/Game/UMG界面/Inventory库存/W_PickupPrompt拾取提示` (`WidgetComponent.GetUserWidgetObject` (`self.PromptWidget提示控件`)) :!pure true) _returnvalue_3)
      (if _returnvalue_3
        (`self.EnableInput` _returnvalue)
        (else
          (`self.DisableInput` _returnvalue)))
      (else
        (`SceneComponent.SetVisibility` `_promptwidget提示控件` false false)
        (`self.DisableInput` (`GameplayStatics.GetPlayerController` 0))))))

(event `InputAction|交互`
  (params (Key :type "Key Structure"))
  (:`Pressed`
    (`self.PickUpItem拾取道具`)))

(fn `PickUpItem拾取道具`
  (returns (`Success成功` :type Boolean))
  (bind (`_success成功` `_remainder余数`) (`/Game/Blueprints蓝图/BlueprintComponents蓝图组件/BPC_Inventory库存组件.AddItem添加道具` (`/Game/GameBP游戏蓝图/Level1关卡1/L1_PlayerCharacter角色.BPC_Inventory库存组件` (`self.PlayerRef角色映射`)) (`self.Item道具`) (`self.Amount数量`)))
  (if `_success成功`
    (if (> `_remainder余数` 0)
      (set `self.Amount数量` `_remainder余数`)
      (return true)
      (else
        (`self.K2_DestroyActor`)
        (return true)))
    (else
      (return false))))

(fn `UserConstructionScript`
  (`SceneComponent.K2_SetRelativeLocation` (`self.PromptWidget提示控件`) (`KismetMathLibrary.MakeVector` 0.0 0.0 (`self.WidgeDistance提示控件距离`)) false false))