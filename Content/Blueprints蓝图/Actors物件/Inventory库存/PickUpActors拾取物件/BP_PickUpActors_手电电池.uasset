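; Flashlight battery pickup actor, a child of a pickup base class that supplies the pickup logic.
; It overrides PickUpItem to call the parent and pass its result back.
; On a successful pickup it sends a task-completion message to the GameState for the "拾取电池" (pick up battery) task and immediately sets the next task.
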(fn `PickUpItem拾取道具`
  (returns (`Success成功` :type Boolean))
  (bind `_success成功` (`parent.PickUpItem拾取道具`))
  (if `_success成功`
    (message `/Game/Blueprints蓝图/Interfaces蓝图接口/BPI_TaskCall任务信息传递.CompleteTaskCall完成任务通知` (`GameplayStatics.GetGameState`) "拾取电池" true)
    (return `_success成功`)
    (else
      (return `_success成功`))))

(fn `UserConstructionScript`
  (`parent.UserConstructionScript`))