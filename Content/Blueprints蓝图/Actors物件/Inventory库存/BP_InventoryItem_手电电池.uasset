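; Flashlight battery inventory item that recharges the player's flashlight when used.
; On use, it adds charge through the player's flashlight component only if the battery is below maximum, and flags whether the use succeeded.
; A successful use also tells the game state to complete the battery-use task without automatically setting the next task.
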(event `self.UsePropEffect使用道具效果`
  (bind `_bpc_flashlight手电筒` (`/Game/GameBP游戏蓝图/Level1关卡1/L1_PlayerCharacter角色.BPC_Flashlight手电筒` (`self.PlayerRef角色映射`)))
  (if (< (`/Game/Blueprints蓝图/BlueprintComponents蓝图组件/BPC_Flashlight手电筒.CurrentBatteryLevel当前电池电量` `_bpc_flashlight手电筒`) (`/Game/Blueprints蓝图/BlueprintComponents蓝图组件/BPC_Flashlight手电筒.MaxBatteryLevel最大电池电量` `_bpc_flashlight手电筒`))
    (`/Game/Blueprints蓝图/BlueprintComponents蓝图组件/BPC_Flashlight手电筒.AddBatteryLife增加电量` `_bpc_flashlight手电筒` (`self.Amount电池增加电量`))
    (set `self.UseItemSuccess使用道具成功` true)
    (message `/Game/Blueprints蓝图/Interfaces蓝图接口/BPI_TaskCall任务信息传递.CompleteTaskCall完成任务通知` (`GameplayStatics.GetGameState`) "使用电池" false)
    (else
      (set `self.UseItemSuccess使用道具成功` false))))

(fn `UserConstructionScript`
  (`parent.UserConstructionScript`))