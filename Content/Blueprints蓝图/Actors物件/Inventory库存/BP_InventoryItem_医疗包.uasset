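; Medkit inventory item Blueprint (医疗包) that restores the player's health when used.
; Its use-prop-effect event checks the player's health component and adds a configurable HP amount only when current health is below the maximum.
; It sets a use-success flag to true when healing happens and false when health is already full.
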(event `self.UsePropEffect使用道具效果`
  (bind `_bpc_health健康` (`/Game/GameBP游戏蓝图/Level1关卡1/L1_PlayerCharacter角色.BPC_health健康` (`self.PlayerRef角色映射`)))
  (if (< (`/Game/Blueprints蓝图/BlueprintComponents蓝图组件/BPC_health健康.CurrentHealth当前健康值` `_bpc_health健康`) (`/Game/Blueprints蓝图/BlueprintComponents蓝图组件/BPC_health健康.MaxHealth最大健康值` `_bpc_health健康`))
    (`/Game/Blueprints蓝图/BlueprintComponents蓝图组件/BPC_health健康.AddHealth增加hp` `_bpc_health健康` (`self.AddHpAmount增加HP数量`))
    (set `self.UseItemSuccess使用道具成功` true)
    (else
      (set `self.UseItemSuccess使用道具成功` false))))

(fn `UserConstructionScript`
  (`parent.UserConstructionScript`))