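; Interactable door actor that swings open or shut each time it is interacted with.
; The Interact event flips a closed-state flag, then plays or reverses a single timeline.
; The timeline's alpha lerps the door mesh's relative yaw between zero and a negative quarter turn, so closing retraces the opening motion.
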(event `/Game/Blueprints蓝图/Interfaces蓝图接口/BPI_interaction交互.interact交互`
  (if (`self.isDoorClosed是否关门`)
    (set `self.isDoorClosed是否关门` false)
    (bind (_direction _alpha) (`Timeline|打开门TL` :!label _label)
      (:`Update`
        (`SceneComponent.K2_SetRelativeRotation` (`self.StaticMesh1`) (`KismetMathLibrary.MakeRotator` 0.0 0.0 (`KismetMathLibrary.Lerp` 0.0 -90.0 _alpha)) false false)))
    (else
      (set `self.isDoorClosed是否关门` true)
      (goto _label :!via `Reverse`))))

(fn `UserConstructionScript`
  (`parent.UserConstructionScript`))