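; BP_LockDial is one rotating dial of a combination lock, with ten digit positions spaced 36 degrees apart.
; On BeginPlay it hands itself to left and right arrow widgets and starts at a random digit.
; A single timeline, played forward or reversed, animates each step while a flag blocks overlapping turns.
; When a turn finishes, it wraps the angle, derives and prints the digit, and has BPLockRef check the lock.
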(event `self.ReceiveBeginPlay`
  (`/Game/UMG界面/W_Arrow箭头按钮.Initialize初始化` (cast `/Game/UMG界面/W_Arrow箭头按钮` (`WidgetComponent.GetUserWidgetObject` (`self.RightArrow右箭头`)) :!pure true) self true)
  (`/Game/UMG界面/W_Arrow箭头按钮.Initialize初始化` (cast `/Game/UMG界面/W_Arrow箭头按钮` (`WidgetComponent.GetUserWidgetObject` (`self.LeftArrow左箭头`)) :!pure true) self false)
  (`self.SetRandomNumber设置随机数`))

(event `FindNumber查找编号`
  (bind _output_get (set `self.Number数字` (`KismetMathLibrary.Abs_Int` (`KismetMathLibrary.FTrunc` (/ (`self.DialRotation刻度盘旋转`) 36.0)))))
  (`KismetSystemLibrary.PrintString` (`KismetStringLibrary.Conv_IntToString` _output_get)))

(event `RotationDial旋转刻度盘`
  (bind `_dialrotation刻度盘旋转` (`self.DialRotation刻度盘旋转`))
  (if (`self.CanRotation可旋转`)
    (set `self.CanRotation可旋转` false)
    (bind (_direction _alpha) (`Timeline|旋转刻度盘` :!via `PlayFromStart` :!label _label)
      (:`Update`
        (bind _returnvalue (+ (`self.DialRotation刻度盘旋转`) (select `ETimelineDirection` _direction :`Forward` (`KismetMathLibrary.Lerp` 0.0 36.0 _alpha) :`Backward` (`KismetMathLibrary.Lerp` -36.0 0.0 _alpha))))
        (`SceneComponent.K2_SetRelativeRotation` (`self.LockDialMesh锁刻度盘`) (`KismetMathLibrary.MakeRotator` 0.0 0.0 _returnvalue) false false))
      (:`Finished`
        (set `self.DialRotation刻度盘旋转` _returnvalue)
        (if (>= `_dialrotation刻度盘旋转` 360.0)
          (set `self.DialRotation刻度盘旋转` 0.0)
          (`SceneComponent.K2_SetRelativeRotation` :`self` (`self.LockDialMesh锁刻度盘`))
          (elif (< `_dialrotation刻度盘旋转` 0.0)
            (bind _output_get (set `self.DialRotation刻度盘旋转` (`KismetMathLibrary.MapRangeClamped` (`self.DialRotation刻度盘旋转`) 0.0 -360.0 360.0)))
            (`SceneComponent.K2_SetRelativeRotation` (`self.LockDialMesh锁刻度盘`) (`KismetMathLibrary.MakeRotator` 0.0 0.0 _output_get) false false)))
        (`self.FindNumber查找编号`)
        (`/Game/Blueprints蓝图/Actors物件/BP_Lock锁.CheckEveryTurn检查每次旋转` (`self.BP_LockRef`))
        (set `self.CanRotation可旋转` true)))))

(event `RotateDialLeft向左旋转刻度盘`
  (if (`self.CanRotation可旋转`)
    (set `self.CanRotation可旋转` false)
    (goto _label :!via `ReverseFromEnd`)))

(fn `SetRandomNumber设置随机数`
  (locals (`LocalRotation局部旋转` :type "Float (double-precision)"))
  (set `local.LocalRotation局部旋转` (* (`KismetMathLibrary.RandomIntegerInRange` 0 9) 36))
  (`SceneComponent.K2_SetRelativeRotation` (`self.LockDialMesh锁刻度盘`) (`KismetMathLibrary.MakeRotator` 0.0 0.0 (`local.LocalRotation局部旋转`)) false false)
  (set `self.DialRotation刻度盘旋转` (`local.LocalRotation局部旋转`))
  (`self.FindNumber查找编号`))

(fn `UserConstructionScript`)