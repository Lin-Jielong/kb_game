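; Interactable hiding spot actor that moves the player into a hide position and back out to an exit position.
; Interact disables the player's collision, movement and inventory access when entering, then starts a looping per-frame timer that slides the character to the target at constant speed.
; On arrival the timers clear, a finished-moving dispatcher fires, and the hiding flag flips, restoring collision, walking and inventory on exit.
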(event `self.ReceiveBeginPlay`
  (bind `_asl1_player_character角色` (cast `/Game/GameBP游戏蓝图/Level1关卡1/L1_PlayerCharacter角色` (`GameplayStatics.GetPlayerCharacter` 0)))
  (set `self.PlayerRef角色映射` `_asl1_player_character角色`)
  (bind `_ashg_player_controller玩家控制器` (cast `/Game/GameBP游戏蓝图/HG_PlayerController玩家控制器` (`GameplayStatics.GetPlayerController` 0)))
  (set `self.ControllerRef控制器映射` `_ashg_player_controller玩家控制器`))

(event `/Game/Blueprints蓝图/Interfaces蓝图接口/BPI_interaction交互.interact交互`
  (bind `_playerref角色映射` (`self.PlayerRef角色映射`))
  (if (`/Game/GameBP游戏蓝图/Level1关卡1/L1_PlayerCharacter角色.IsHiding正在隐藏` (`self.PlayerRef角色映射`))
    (bind _returnvalue (`KismetSystemLibrary.K2_SetTimerDelegate` (delegate `MoveCharacter移动角色`) (`GameplayStatics.GetWorldDeltaSeconds`) true))
    (else
      (`self.SetActorEnableCollision` `_playerref角色映射` false)
      (`CharacterMovementComponent.DisableMovement` (`Character.CharacterMovement` `_playerref角色映射`))
      (set `/Game/GameBP游戏蓝图/HG_PlayerController玩家控制器.CanOpenInventory可打开库存` false (`self.ControllerRef控制器映射`))
      (bind _returnvalue_2 (`KismetSystemLibrary.K2_SetTimerDelegate` (delegate `MoveCharacter移动角色`) (`GameplayStatics.GetWorldDeltaSeconds`) true)))))

(event `MoveCharacter移动角色`
  (bind `_playerref角色映射` (`self.PlayerRef角色映射`))
  (`self.K2_SetActorTransform` `_playerref角色映射` (`KismetMathLibrary.MakeTransform` (`KismetMathLibrary.VInterpTo_Constant` (`self.K2_GetActorLocation` `_playerref角色映射`) (`SceneComponent.K2_GetComponentLocation` (select `bool` (`/Game/GameBP游戏蓝图/Level1关卡1/L1_PlayerCharacter角色.IsHiding正在隐藏` (`self.PlayerRef角色映射`)) :`false` (`self.HidePosition隐藏位置`) :`true` (`self.ExitPosition出口位置`) :!type "SceneComponent Object Reference")) (`GameplayStatics.GetWorldDeltaSeconds`) 1000.0)) false false)
  (if (== (`self.K2_GetActorLocation` (`self.PlayerRef角色映射`)) (`SceneComponent.K2_GetComponentLocation` (select `bool` (`/Game/GameBP游戏蓝图/Level1关卡1/L1_PlayerCharacter角色.IsHiding正在隐藏` (`self.PlayerRef角色映射`)) :`false` (`self.HidePosition隐藏位置`) :`true` (`self.ExitPosition出口位置`) :!type "SceneComponent Object Reference")) :`ErrorTolerance` 0.01)
    (`KismetSystemLibrary.K2_ClearAndInvalidateTimerHandle` (stale `/Game/Blueprints蓝图/Interfaces蓝图接口/BPI_interaction交互.interact交互` _returnvalue_2))
    (`KismetSystemLibrary.K2_ClearAndInvalidateTimerHandle` (stale `/Game/Blueprints蓝图/Interfaces蓝图接口/BPI_interaction交互.interact交互` _returnvalue))
    (`self.FinishedMoving完成移动`)))

(event `FinishedMoving完成移动`
  (bind `_playerref角色映射` (`self.PlayerRef角色映射`))
  (bind `_playerref角色映射_2` (`self.PlayerRef角色映射`))
  (`self.FinishedMovingED完成移动`)
  (if (`/Game/GameBP游戏蓝图/Level1关卡1/L1_PlayerCharacter角色.IsHiding正在隐藏` `_playerref角色映射`)
    (set `/Game/GameBP游戏蓝图/Level1关卡1/L1_PlayerCharacter角色.IsHiding正在隐藏` false `_playerref角色映射`)
    (`self.SetActorEnableCollision` `_playerref角色映射_2` true)
    (`CharacterMovementComponent.SetMovementMode` (`Character.CharacterMovement` `_playerref角色映射_2`) "MOVE_Walking" 0)
    (set `/Game/GameBP游戏蓝图/HG_PlayerController玩家控制器.CanOpenInventory可打开库存` true (`self.ControllerRef控制器映射`))
    (else
      (set `/Game/GameBP游戏蓝图/Level1关卡1/L1_PlayerCharacter角色.IsHiding正在隐藏` true `_playerref角色映射`))))

(fn `UserConstructionScript`)