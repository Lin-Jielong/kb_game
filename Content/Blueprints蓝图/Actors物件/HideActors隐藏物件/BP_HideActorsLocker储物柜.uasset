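; Locker hiding-spot actor that adds an animated swinging door to its parent hide-actor behaviour.
; Interact is gated by a can-interact flag, plays an open timeline rotating the door mesh's yaw, then calls the parent Interact after a short delay.
; The FinishedMovingED event triggers a delayed CloseDoor, whose separate timeline swings the door back and re-enables interaction when finished.
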(event `self.ReceiveBeginPlay`
  (`parent.ReceiveBeginPlay`)
  (add `self.FinishedMovingED完成移动` (delegate `FinishedMovingED完成移动_事件_0`)))

(event `FinishedMovingED完成移动_事件_0`
  (`KismetSystemLibrary.Delay` 0.1)
  (`self.CloseDoor关门`))

(event `/Game/Blueprints蓝图/Interfaces蓝图接口/BPI_interaction交互.interact交互`
  (if (`self.CanInteract可交互`)
    (set `self.CanInteract可交互` false)
    (bind (_direction _alpha) (`Timeline|打开储物门` :!via `PlayFromStart`)
      (:`Update`
        (`SceneComponent.K2_SetRelativeRotation` (`self.StaticMesh1`) (`KismetMathLibrary.MakeRotator` 0.0 0.0 (`KismetMathLibrary.Lerp` -90.0 0.0 _alpha)) false false))
      (:`Finished`
        (`KismetSystemLibrary.Delay` 0.1)
        (`parent.interact交互`)))))

(event `CloseDoor关门`
  (bind (_direction _alpha) (`Timeline|关闭储物门` :!via `PlayFromStart`)
    (:`Update`
      (`SceneComponent.K2_SetRelativeRotation` (`self.StaticMesh1`) (`KismetMathLibrary.MakeRotator` 0.0 0.0 (`KismetMathLibrary.Lerp` 0.0 -90.0 _alpha)) false false))
    (:`Finished`
      (set `self.CanInteract可交互` true))))

(fn `UserConstructionScript`
  (`parent.UserConstructionScript`))