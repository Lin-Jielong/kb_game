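; BPC_health is a health component that tracks current health and drives a blood-screen effect.
; Add and remove functions change health within its minimum and maximum bounds, then refresh the effect, which also updates on BeginPlay.
; The refresh writes a clamped, remapped health value to a Material Parameter Collection scalar, so it varies only below 70% of maximum health.
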(event `self.ReceiveBeginPlay`
  (`self.UpdateBloodScreen更新血屏`))

(fn `AddHealth增加hp`
  (params (`Amount数量 ` :type "Float (double-precision)"))
  (set `self.CurrentHealth当前健康值` (`KismetMathLibrary.FClamp` (+ (`self.CurrentHealth当前健康值`) `Amount数量 `) (`self.MinHealth最小健康值`) (`self.MaxHealth最大健康值`)))
  (`self.UpdateBloodScreen更新血屏`))

(fn `RemoveHealth减少hp`
  (params (`Amount数量 ` :type "Float (double-precision)"))
  (set `self.CurrentHealth当前健康值` (`KismetMathLibrary.FClamp` (- (`self.CurrentHealth当前健康值`) `Amount数量 `) (`self.MinHealth最小健康值`) (`self.MaxHealth最大健康值`)))
  (`self.UpdateBloodScreen更新血屏`))

(fn `UpdateBloodScreen更新血屏`
  (`KismetMaterialLibrary.SetScalarParameterValue` "/Game/Props道具/Materials材质/MPC_BloodScreen血屏.MPC_BloodScreen血屏" "Amount数量" (`KismetMathLibrary.MapRangeClamped` (`self.CurrentHealth当前健康值`) (`self.MinHealth最小健康值`) (* (`self.MaxHealth最大健康值`) 0.7) 0.5 1.0)))