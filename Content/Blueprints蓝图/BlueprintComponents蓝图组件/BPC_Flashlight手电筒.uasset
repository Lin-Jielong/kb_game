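; Flashlight component that gives the player a toggleable light powered by a draining battery.
; Initialize caches the player and its Flashlight light; toggling on requires charge and starts a looping timer, by function name, that depletes the battery and switches the light off when empty.
; AddBatteryLife recharges within clamped limits.
; Battery changes remap charge to the light's IES brightness scale, so dimming occurs only below a fixed low-charge threshold.
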(fn `AddBatteryLife增加电量`
  (params (`Amount数量` :type "Float (double-precision)"))
  (set `self.CurrentBatteryLevel当前电池电量` (`KismetMathLibrary.FClamp` (+ `Amount数量` (`self.CurrentBatteryLevel当前电池电量`)) (`self.MinBatteryLevel最小电池电量`) (`self.MaxBatteryLevel最大电池电量`)))
  (`self.SetIntensity设置强度`))

(fn `Deplete Battery Life消耗电量`
  (set `self.CurrentBatteryLevel当前电池电量` (`KismetMathLibrary.FClamp` (- (`self.CurrentBatteryLevel当前电池电量`) (`self.DepleteAmount消耗电量`)) (`self.MinBatteryLevel最小电池电量`) (`self.MaxBatteryLevel最大电池电量`)))
  (`self.SetIntensity设置强度`)
  (if (<= (`self.CurrentBatteryLevel当前电池电量`) (`self.MinBatteryLevel最小电池电量`))
    (`SceneComponent.SetVisibility` (`self.Flashlight手电光源`) false false)
    (`KismetSystemLibrary.K2_ClearTimer` null "Deplete Battery Life消耗电量")))

(fn `Initialize初始化`
  (params (`player角色` :type "/Game/GameBP游戏蓝图/Level1关卡1/L1_PlayerCharacter角色 Object Reference"))
  (bind _output_get (set `self.Player角色` `player角色`))
  (set `self.Flashlight手电光源` (`/Game/GameBP游戏蓝图/Level1关卡1/L1_PlayerCharacter角色.Flashlight` _output_get)))

(fn `SetIntensity设置强度`
  (`LightComponent.SetIESBrightnessScale` (`self.Flashlight手电光源`) (`KismetMathLibrary.MapRangeClamped` (`self.CurrentBatteryLevel当前电池电量`) (`self.MinBatteryLevel最小电池电量`) 20.0 0.0 1.0)))

(fn `ToggleFlashlight切换手电筒`
  (bind `_flashlight手电光源` (`self.Flashlight手电光源`))
  (if (`SceneComponent.bVisible` `_flashlight手电光源`)
    (`SceneComponent.SetVisibility` `_flashlight手电光源` false false)
    (`KismetSystemLibrary.K2_ClearTimer` null "Deplete Battery Life消耗电量")
    (elif (> (`self.CurrentBatteryLevel当前电池电量`) (`self.MinBatteryLevel最小电池电量`))
      (`self.SetIntensity设置强度`)
      (`SceneComponent.SetVisibility` `_flashlight手电光源` true false)
      (`KismetSystemLibrary.K2_SetTimer` null "Deplete Battery Life消耗电量" (`self.Speed速度`) true))))