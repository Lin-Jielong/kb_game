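; Inventory component that stores the player's items in a slot array, sized from the player controller and expandable at runtime.
; Adding fills partial stacks, then empty slots, recursing on overflow and returning any remainder.
; Using an item runs its effect on an existing or spawned actor, removing one on success.
; Dropping spawns a physics pickup of the whole stack via camera trace; slot changes refresh the inventory grid widget.
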(event `self.ReceiveBeginPlay`
  (bind `_ashg_player_controller玩家控制器` (cast `/Game/GameBP游戏蓝图/HG_PlayerController玩家控制器` (`GameplayStatics.GetPlayerController` 0) :!pure true))
  (`KismetArrayLibrary.Array_Resize` (`self.InventorySlots库存格子`) (`/Game/GameBP游戏蓝图/HG_PlayerController玩家控制器.InventorySlots库存格子` `_ashg_player_controller玩家控制器`))
  (set `self.W Inventory Menu Ref库存菜单映射` (`/Game/GameBP游戏蓝图/HG_PlayerController玩家控制器.W_InventoryMenuRef库存菜单映射` `_ashg_player_controller玩家控制器`))
  (bind `_asl1_player_character角色` (cast `/Game/GameBP游戏蓝图/Level1关卡1/L1_PlayerCharacter角色` (`GameplayStatics.GetPlayerCharacter` 0)))
  (set `self.PlayerRef角色映射` `_asl1_player_character角色`)
  (bind _outactors (`GameplayStatics.GetAllActorsOfClass` "/Game/Blueprints蓝图/Actors物件/Inventory库存/BP_Examination查看.BP_Examination查看_C"))
  (set `self.ExaminationRef查看映射` (`|GetArrayItem` _outactors)))

(fn `AddItemSlots添加道具格子`
  (params (`Amount数量` :type Integer))
  (bind `_w_inventory_menu_ref库存菜单映射` (`self.W Inventory Menu Ref库存菜单映射`))
  (bind `_ashg_player_controller玩家控制器` (cast `/Game/GameBP游戏蓝图/HG_PlayerController玩家控制器` (`GameplayStatics.GetPlayerController` 0) :!pure true))
  (bind `_w_inventorygrid库存网格` (`/Game/UMG界面/Inventory库存/W_InventoryMenu库存菜单.W_InventoryGrid库存网格` `_w_inventory_menu_ref库存菜单映射`))
  (bind _output_get (set `/Game/GameBP游戏蓝图/HG_PlayerController玩家控制器.InventorySlots库存格子` (+ `Amount数量` (`/Game/GameBP游戏蓝图/HG_PlayerController玩家控制器.InventorySlots库存格子` `_ashg_player_controller玩家控制器`)) `_ashg_player_controller玩家控制器`))
  (`KismetArrayLibrary.Array_Resize` (`self.InventorySlots库存格子`) _output_get)
  (`/Game/UMG界面/Inventory库存/W_InventoryGrid库存网格.AddMoreSlots添加格子` `_w_inventorygrid库存网格` `Amount数量`)
  (for _array_element (`/Game/UMG界面/Inventory库存/W_InventoryGrid库存网格.SlotsArray格子数组` `_w_inventorygrid库存网格`)
    (`/Game/UMG界面/Inventory库存/W_InventorySlot库存格子.Initialize初始化` _array_element `_w_inventory_menu_ref库存菜单映射`)))

(fn `AddItem添加道具`
  (params (`Item道具` :type "/Game/Blueprints蓝图/Actors物件/Inventory库存/BP_InventoryItem_Master库存道具主类 Class Reference") (`Amount数量` :type Integer))
  (returns (`Success成功` :type Boolean) (`Remainder余数` :type Integer))
  (locals (`LocalItem局部道具` :type "/Game/Blueprints蓝图/Actors物件/Inventory库存/BP_InventoryItem_Master库存道具主类 Class Reference") (`LocalAmount局部数量` :type Integer) (`LocalMaxStackAmount局部叠加数` :type Integer) (`LocalIndex局部索引` :type Integer :default 0))
  (bind (`_success成功` `_index索引`) (`self.CheckForEmptySlot查找空格子`))
  (bind (`_success成功_2` `_index索引_2`) (`self.CheckForEmptySlot查找空格子`))
  (bind _returnvalue (- (`local.LocalAmount局部数量`) 1))
  (bind (`_itemname道具名称` `_icon图标` `_maxstackamount最大叠加数`) (break `/Game/Blueprints蓝图/Structs结构/S_ItemData道具数据_2` (`.ItemDate道具数据` (defaults `Object` (`local.LocalItem局部道具`)))))
  (set `local.LocalItem局部道具` `Item道具`)
  (set `local.LocalAmount局部数量` `Amount数量`)
  (set `local.LocalMaxStackAmount局部叠加数` `_maxstackamount最大叠加数`)
  (if (> `_maxstackamount最大叠加数` 1)
    (bind (`_success成功_3` `_index索引_3`) (`self.CheckForFreeSlot查找有空间格子` (`local.LocalItem局部道具`)))
    (if `_success成功_3`
      (set `local.LocalIndex局部索引` `_index索引_3`)
      (bind _returnvalue_2 (+ (`.Amount数量` (`self.GetItemDataAtIndex获取道具数据索引` `_index索引_3`)) (`local.LocalAmount局部数量`)))
      (if (> _returnvalue_2 (`local.LocalMaxStackAmount局部叠加数`))
        (set `local.LocalAmount局部数量` (- _returnvalue_2 (`local.LocalMaxStackAmount局部叠加数`)))
        (`KismetArrayLibrary.Array_Set` (`self.InventorySlots库存格子`) (`local.LocalIndex局部索引`) (make `/Game/Blueprints蓝图/Structs结构/S_InventoryItem库存道具` (`local.LocalItem局部道具`) (`local.LocalMaxStackAmount局部叠加数`)))
        (`self.UpdateInventorySlot更新库存格子` (`local.LocalIndex局部索引`))
        (bind (`_success成功_4` `_remainder余数`) (`self.AddItem添加道具` (`local.LocalItem局部道具`) (`local.LocalAmount局部数量`)))
        (return true `_remainder余数`)
        (else
          (`KismetArrayLibrary.Array_Set` (`self.InventorySlots库存格子`) (`local.LocalIndex局部索引`) (make `/Game/Blueprints蓝图/Structs结构/S_InventoryItem库存道具` (`local.LocalItem局部道具`) _returnvalue_2))
          (`self.UpdateInventorySlot更新库存格子` (`local.LocalIndex局部索引`))
          (return true 0)))
      (elif `_success成功_2`
        (set `local.LocalIndex局部索引` `_index索引_2`)
        (if (> (`local.LocalAmount局部数量`) (`local.LocalMaxStackAmount局部叠加数`))
          ;[1 1 1] 当拾取的物品叠加数大于该物品最大叠加数时，有多少存多少，剩余的再循环一次添加道具逻辑
          (`KismetArrayLibrary.Array_Set` (`self.InventorySlots库存格子`) (`local.LocalIndex局部索引`) (make `/Game/Blueprints蓝图/Structs结构/S_InventoryItem库存道具` (`local.LocalItem局部道具`) (`local.LocalMaxStackAmount局部叠加数`)))
          (`self.UpdateInventorySlot更新库存格子` (`local.LocalIndex局部索引`))
          (bind (`_success成功_5` `_remainder余数_2`) (`self.AddItem添加道具` (`local.LocalItem局部道具`) (- (`local.LocalAmount局部数量`) (`local.LocalMaxStackAmount局部叠加数`))))
          (return true `_remainder余数_2`)
          (else
            ;[1 1 1] 当拾取的道具小于最大叠加数，直接找空格子添加
            (`KismetArrayLibrary.Array_Set` (`self.InventorySlots库存格子`) (`local.LocalIndex局部索引`) (make `/Game/Blueprints蓝图/Structs结构/S_InventoryItem库存道具` (`local.LocalItem局部道具`) (`local.LocalAmount局部数量`)))
            (`self.UpdateInventorySlot更新库存格子` (`local.LocalIndex局部索引`))
            (return true 0)))
        (else
          (return false (`local.LocalAmount局部数量`)))))
    (elif `_success成功`
      (set `local.LocalIndex局部索引` `_index索引`)
      (`KismetArrayLibrary.Array_Set` (`self.InventorySlots库存格子`) (`local.LocalIndex局部索引`) (make `/Game/Blueprints蓝图/Structs结构/S_InventoryItem库存道具` (`local.LocalItem局部道具`) 1))
      (`self.UpdateInventorySlot更新库存格子` (`local.LocalIndex局部索引`))
      (if (> _returnvalue 0)
        (bind (`_success成功_6` `_remainder余数_3`) (`self.AddItem添加道具` (`local.LocalItem局部道具`) _returnvalue))
        (return true `_remainder余数_3`)
        (else
          (return true 0)))
      (else
        (`KismetSystemLibrary.PrintString` "背包已经满了")
        (return false (`local.LocalAmount局部数量`))))))

(fn `CheckForEmptySlot查找空格子`
  (returns (`Success成功` :type Boolean) (`Index索引` :type Integer))
  (locals (`LocalSuccess局部成功` :type Boolean) (`Localindex局部索引` :type Integer))
  (for (_array_element _array_index) (`self.InventorySlots库存格子`)
    (if (`KismetSystemLibrary.IsValidClass` (`.Item道具_2_7B9726DB4EF2FB6E7F2DD0AA2B696C22` (break `/Game/Blueprints蓝图/Structs结构/S_InventoryItem库存道具` _array_element)))
      (set `local.LocalSuccess局部成功` false)
      (else
        (set `local.LocalSuccess局部成功` true)
        (set `local.Localindex局部索引` _array_index)
        (break))))
  (return (`local.LocalSuccess局部成功`) (`local.Localindex局部索引`)))

(fn `CheckForFreeSlot查找有空间格子`
  (params (`Item道具` :type "/Game/Blueprints蓝图/Actors物件/Inventory库存/BP_InventoryItem_Master库存道具主类 Class Reference"))
  (returns (`Success成功` :type Boolean) (`Index索引` :type Integer))
  (locals (`LocalSuccess局部成功` :type Boolean) (`LocalIndex局部索引` :type Integer))
  (for (_array_element _array_index) (`self.InventorySlots库存格子`)
    (bind (`_item道具` `_amoult数量`) (break `/Game/Blueprints蓝图/Structs结构/S_InventoryItem库存道具` _array_element))
    (if (and (== `_item道具` `Item道具`) (< `_amoult数量` (`.MaxStackAmount最大叠加数_8_6E00D90643B2F63EB00D80AD9E320078` (break `/Game/Blueprints蓝图/Structs结构/S_ItemData道具数据_2` (`.ItemDate道具数据` (defaults `Object` `Item道具`))))))
      (set `local.LocalSuccess局部成功` true)
      (set `local.LocalIndex局部索引` _array_index)
      (break)
      (else
        (set `local.LocalSuccess局部成功` false))))
  (return (`local.LocalSuccess局部成功`) (`local.LocalIndex局部索引`)))

(fn `DropItem丢弃道具`
  (params (`Index索引` :type Integer))
  (locals (`LocalIndex局部索引` :type Integer) (`LocalAmount局部数量` :type Integer :default 0) (`LocalItem局部道具` :type "/Game/Blueprints蓝图/Actors物件/Inventory库存/BP_InventoryItem_Master库存道具主类 Class Reference"))
  (bind _camera (`/Game/GameBP游戏蓝图/Level1关卡1/L1_PlayerCharacter角色.Camera` (`self.PlayerRef角色映射`)))
  (bind _returnvalue (`SceneComponent.K2_GetComponentLocation` _camera))
  (bind _output_get (set `local.LocalIndex局部索引` `Index索引`))
  (bind (`_item道具` `_amount数量`) (`self.GetItemDataAtIndex获取道具数据索引` _output_get))
  (set `local.LocalAmount局部数量` `_amount数量`)
  (set `local.LocalItem局部道具` `_item道具`)
  (if (> (`local.LocalAmount局部数量`) 0)
    (for _ (range (`local.LocalAmount局部数量`))
      (`self.RemoveItem移除道具` (`local.LocalIndex局部索引`)))
    (`/Game/UMG界面/Inventory库存/W_InventoryMenu库存菜单.CloseItemInfo关闭道具信息` (`self.W Inventory Menu Ref库存菜单映射`))
    (bind (_outhit _returnvalue_2) (`KismetSystemLibrary.LineTraceSingle` _returnvalue (+ _returnvalue (* (`SceneComponent.GetForwardVector` _camera) 200)) "TraceTypeQuery1"))
    (bind (_bblockinghit _binitialoverlap _time _distance _location _impactpoint _normal _impactnormal _physmat _hitactor _hitcomponent _hitbonename _bonename _hititem _elementindex _faceindex _tracestart _traceend) (`GameplayStatics.BreakHitResult` _outhit))
    (bind _returnvalue_3 (`|SpawnActorFromClass` (`.PickUpItem拾取物品_30_90BC5E9246728782AE02DC9D73033671` (break `/Game/Blueprints蓝图/Structs结构/S_ItemData道具数据_2` (`.ItemDate道具数据` (defaults `Object` (`local.LocalItem局部道具`))))) (`KismetMathLibrary.MakeTransform` (select `bool` _returnvalue_2 :`false` _traceend :`true` _location)) "Undefined" "OverrideRootScale" null false null))
    (set `/Game/Blueprints蓝图/Actors物件/Inventory库存/PickUpActors拾取物件/BP_PickUpActors_Master拾取物品主类.Amount数量` (`local.LocalAmount局部数量`) _returnvalue_3)
    (`PrimitiveComponent.SetSimulatePhysics` (`/Game/Blueprints蓝图/Actors物件/Inventory库存/PickUpActors拾取物件/BP_PickUpActors_Master拾取物品主类.StaticMesh` _returnvalue_3) true)))

(fn `GetItemDataAtIndex获取道具数据索引`
  (params (`Index索引` :type Integer))
  (returns (`Item道具` :type "/Game/Blueprints蓝图/Actors物件/Inventory库存/BP_InventoryItem_Master库存道具主类 Class Reference") (`Amount数量` :type Integer))
  (bind (`_item道具` `_amoult数量`) (break `/Game/Blueprints蓝图/Structs结构/S_InventoryItem库存道具` (`|GetArrayItem` (`self.InventorySlots库存格子`) `Index索引`)))
  (return `_item道具` `_amoult数量`))

(fn `RemoveItem移除道具`
  (params (`Index索引` :type Integer))
  (bind (`_item道具` `_amount数量`) (`self.GetItemDataAtIndex获取道具数据索引` `Index索引`))
  (bind `_inventoryslots库存格子` (`self.InventorySlots库存格子`))
  (if (> `_amount数量` 1)
    (`KismetArrayLibrary.Array_Set` `_inventoryslots库存格子` `Index索引` (make `/Game/Blueprints蓝图/Structs结构/S_InventoryItem库存道具` `_item道具` (- `_amount数量` 1)))
    (else
      (`KismetArrayLibrary.Array_Set` `_inventoryslots库存格子` `Index索引`)))
  (`self.UpdateInventorySlot更新库存格子` `Index索引`))

(fn `UpdateInventorySlot更新库存格子`
  (params (`Index索引` :type Integer))
  (`/Game/UMG界面/Inventory库存/W_InventorySlot库存格子.UpDate更新数据` (`|GetArrayItem` (`/Game/UMG界面/Inventory库存/W_InventoryGrid库存网格.SlotsArray格子数组` (`/Game/UMG界面/Inventory库存/W_InventoryMenu库存菜单.W_InventoryGrid库存网格` (`/Game/GameBP游戏蓝图/HG_PlayerController玩家控制器.W_InventoryMenuRef库存菜单映射` (cast `/Game/GameBP游戏蓝图/HG_PlayerController玩家控制器` (`GameplayStatics.GetPlayerController` 0) :!pure true)))) `Index索引`)))

(fn `UseItem使用道具`
  (params (`Index索引` :type Integer))
  (locals (`LocalIndex局部索引` :type Integer) (`Loca局部数量` :type Integer :default 0))
  (bind _output_get (set `local.LocalIndex局部索引` `Index索引`))
  (bind (`_item道具` `_amount数量`) (`self.GetItemDataAtIndex获取道具数据索引` _output_get))
  (set `local.Loca局部数量` `_amount数量`)
  (if (> `_amount数量` 0)
    (bind _returnvalue (`GameplayStatics.GetActorOfClass` `_item道具`))
    (`/Engine/EditorBlueprintResources/StandardMacros.IsValid` _returnvalue
      (:`Is Valid`
        (`/Game/Blueprints蓝图/Actors物件/Inventory库存/BP_InventoryItem_Master库存道具主类.UsePropEffect使用道具效果` _returnvalue)
        (if (`/Game/Blueprints蓝图/Actors物件/Inventory库存/BP_InventoryItem_Master库存道具主类.UseItemSuccess使用道具成功` _returnvalue)
          (`self.RemoveItem移除道具` (`local.LocalIndex局部索引`) :!label _label)
          (if (<= (`local.Loca局部数量`) 1)
            (`/Game/UMG界面/Inventory库存/W_InventoryMenu库存菜单.CloseItemInfo关闭道具信息` (`self.W Inventory Menu Ref库存菜单映射`)))))
      (:`Is Not Valid`
        (bind _returnvalue_2 (`|SpawnActorFromClass` `_item道具` (`KismetMathLibrary.MakeTransform` (0.0 0.0 0.0)) "Undefined" "OverrideRootScale" null null))
        (`/Game/Blueprints蓝图/Actors物件/Inventory库存/BP_InventoryItem_Master库存道具主类.UsePropEffect使用道具效果` _returnvalue_2)
        (if (`/Game/Blueprints蓝图/Actors物件/Inventory库存/BP_InventoryItem_Master库存道具主类.UseItemSuccess使用道具成功` _returnvalue_2)
          (goto _label))))))