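; Player movement component that switches the character's max walk speed between walking, crouching and sprinting, with sprint limited by stamina.
; Crouching stops the sprint drain timer and calls the player character to shrink its capsule; standing restores both capsule and walk speed.
; Looping timers drain stamina while sprinting and moving, then refill it after a retriggerable delay once sprint stops.
; Starting a sprint cancels crouch and, given stamina and movement, halts regeneration.
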(event `StartSprint开始冲刺`
  (if (`self.isCrouching是否蹲着`)
    (`self. EndCrouch结束下蹲`))
  (if (and (> (`self.CurrentStamina当前耐力`) (`self.MinStamina最小耐力`)) (> (`KismetMathLibrary.VSize` (`Actor.GetVelocity` (`self.PlayerRef玩家映射`))) 10.0))
    (`KismetSystemLibrary.K2_ClearTimer` null "RegenerateStamina回复耐力")
    (`self.SetPlayerMaxWalkSpeed玩家移动最大速度` (`self.SprintSpeed冲刺速度`))
    (`KismetSystemLibrary.K2_SetTimer` null "SprintTimer冲刺计时" 0.1 true)))

(event `SprintTimer冲刺计时`
  (if (> (`KismetMathLibrary.VSize` (`Actor.GetVelocity` (`self.PlayerRef玩家映射`))) 10.0)
    (set `self.CurrentStamina当前耐力` (`KismetMathLibrary.FClamp` (- (`self.CurrentStamina当前耐力`) 1.0) (`self.MinStamina最小耐力`) (`self.MaxStamina最大耐力`)))
    (if (<= (`self.CurrentStamina当前耐力`) (`self.MinStamina最小耐力`))
      (`self.StopSprint停止冲刺`))
    (else
      (`self.StopSprint停止冲刺`))))

(event `StopSprint停止冲刺`
  (if (not (`self.isCrouching是否蹲着`))
    (`KismetSystemLibrary.K2_ClearTimer` null "SprintTimer冲刺计时")
    (`self.SetPlayerMaxWalkSpeed玩家移动最大速度` (`self.WalkSpeed行走速度`))
    (`KismetSystemLibrary.RetriggerableDelay` 5.0)
    (if (not (`KismetSystemLibrary.K2_IsTimerActive` null "SprintTimer冲刺计时"))
      (`KismetSystemLibrary.K2_SetTimer` null "RegenerateStamina回复耐力" 0.03 true))))

(event `RegenerateStamina回复耐力`
  (set `self.CurrentStamina当前耐力` (`KismetMathLibrary.FClamp` (+ (`self.CurrentStamina当前耐力`) 1.0) (`self.MinStamina最小耐力`) (`self.MaxStamina最大耐力`)))
  (if (>= (`self.CurrentStamina当前耐力`) (`self.MaxStamina最大耐力`))
    (`KismetSystemLibrary.K2_ClearTimer` null "RegenerateStamina回复耐力")))

(event `StartCouch开始蹲下`
  (`KismetSystemLibrary.K2_ClearTimer` null "SprintTimer冲刺计时")
  (`self.SetPlayerMaxWalkSpeed玩家移动最大速度` (`self.CrouchSpeed下蹲速度`))
  (`/Game/GameBP游戏蓝图/Level1关卡1/L1_PlayerCharacter角色.ShortenPlayerCapsule缩放胶囊体` (cast `/Game/GameBP游戏蓝图/Level1关卡1/L1_PlayerCharacter角色` (`self.PlayerRef玩家映射`) :!pure true))
  (set `self.isCrouching是否蹲着` true))

(event `EndCrouch结束下蹲`
  (`self.SetPlayerMaxWalkSpeed玩家移动最大速度` (`self.WalkSpeed行走速度`))
  (`/Game/GameBP游戏蓝图/Level1关卡1/L1_PlayerCharacter角色.LengthenPlayerCapsule加长胶囊体` (cast `/Game/GameBP游戏蓝图/Level1关卡1/L1_PlayerCharacter角色` (`self.PlayerRef玩家映射`) :!pure true))
  (set `self.isCrouching是否蹲着` false))

(fn `Initialize初始化`
  (params (`Character角色` :type "Character Object Reference"))
  (set `self.PlayerRef玩家映射` `Character角色`)
  (`self.SetPlayerMaxWalkSpeed玩家移动最大速度` (`self.WalkSpeed行走速度`)))

(fn `SetPlayerMaxWalkSpeed玩家移动最大速度`
  (params (`最大行走速度` :type "Float (single-precision)"))
  (set `CharacterMovementComponent.MaxWalkSpeed` `最大行走速度` (`Character.CharacterMovement` (`self.PlayerRef玩家映射`))))